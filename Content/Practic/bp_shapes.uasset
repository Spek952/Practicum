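; Construction-script Blueprint that arranges copies of a chosen static mesh in a ring or open arc around the actor.
; It adds a clamped number of mesh components, rotating a radius vector by even yaw steps, with GapSize widening the opening in the ring.
; Each mesh can follow its angle around the center, plus a yaw offset and shared scale.
; The event graph holds only disabled stubs, so nothing runs during play.
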(fn `UserConstructionScript`
  (bind _number_of_meshes (`self.Number of meshes`))
  (set `self.Number of meshes` (`KismetMathLibrary.Clamp` (`self.Number of meshes`) 1 1000))
  (for _index (range _number_of_meshes)
    (bind _returnvalue (`KismetMathLibrary.MakeRotator` 0.0 0.0 (* _index (/ 360.0 (`KismetMathLibrary.Conv_IntToDouble` (+ _number_of_meshes (`self.GapSize`)))))))
    (bind _returnvalue_2 (`AddComponent|NODE_AddStaticMeshComponent-0` :`RelativeTransform` (`KismetMathLibrary.MakeTransform` (`KismetMathLibrary.GreaterGreater_VectorRotator` (`KismetMathLibrary.MakeVector` (`self.Radius`)) _returnvalue) (`KismetMathLibrary.MakeRotator` (.roll (`KismetMathLibrary.SelectRotator` _returnvalue (struct) (`self.Orient ro center`))) (.pitch (`KismetMathLibrary.SelectRotator` _returnvalue (struct) (`self.Orient ro center`))) (+ (.yaw (`KismetMathLibrary.SelectRotator` _returnvalue (struct) (`self.Orient ro center`))) (`self.Yaw Offset`))) (`self.Mash Scale`))))
    (`StaticMeshComponent.SetStaticMesh` _returnvalue_2 (`self.Mesh to spawn`))))